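; P-38 aircraft actor Blueprint that flies itself forward while rolling, with both propellers spinning.
; Each Tick, a per-second propeller speed variable is scaled by delta seconds and applied as local roll to the Left and Right components.
; The actor also moves along its local X axis and rolls at fixed, frame-rate-independent rates.
; An unconnected node that rotates both propellers in one call remains as a discouraged alternative.
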(event `self.ReceiveTick`
  (params (DeltaSeconds :type "Float (single-precision)"))
  ;[1 1 1] 한프레임당회전속도구하기
  (set `self.한프레임당회전하는속력` (* (`self.1초당프로펠러회전속력`) (`GameplayStatics.GetWorldDeltaSeconds`)))
  ;[1 1 1] 같은 것이라도 따로따로 해야한다. 로컬은 자기 기준 - 물체를 회전시킬때는 loca 아니면 relative로 한다.
  ;;[1 1 1] 왼쪽프로펠러회전시키기
  (`SceneComponent.K2_AddLocalRotation` (`self.Left`) (`KismetMathLibrary.MakeRotator` (`self.한프레임당회전하는속력`)) false false)
  ;;[1 1 1] 오른쪽프로펠러회전시키기
  (`SceneComponent.K2_AddLocalRotation` (`self.Right`) (`KismetMathLibrary.MakeRotator` (`self.한프레임당회전하는속력`)) false false)
  ;[1 1 1] 비행기 본체가 앞으로 이동 (Target 지정할 필요가 없다)
  (`self.K2_AddActorLocalOffset` (`KismetMathLibrary.MakeVector` (* (`GameplayStatics.GetWorldDeltaSeconds`) 30.0)))
  ;[1 1 1] 비행기 본체가 회전
  (`self.K2_AddActorLocalRotation` (`KismetMathLibrary.MakeRotator` (* (`GameplayStatics.GetWorldDeltaSeconds`) 50.0))))

(fn `UserConstructionScript`)